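; Child player projectile that damages NPCs it overlaps.
; On overlap it runs the parent logic, then casts the other actor to BP_NPC, applies Damage through TakeDamage and destroys itself.
; A failed cast only prints a debug message.
; HandleOtherOverlap is unfinished and never called: it compares against the projectile and player, but its destroy step is disconnected.
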(event EventBeginPlay
  (|CallParentFunction) ; This node is disabled and will not be called.\nDrag off pins to build functionality.
)

(event Collision|EventActorBeginOverlap
  (params (OtherActor :type Actor%20Object%20Reference))
  (|CallParentFunction OtherActor)
  (CallFunction|HandleNPCOverlap OtherActor))

(event EventTick
  (params (DeltaSeconds :type Float%20%28single-precision%29))
  (|CallParentFunction DeltaSeconds) ; This node is disabled and will not be called.\nDrag off pins to build functionality.
)

(fn ConstructionScript
  (|CallParentFunction))

(fn HandleNPCOverlap
  (params (Actor :type Actor%20Object%20Reference))
  (bind _asbp_npc (Utilities|Casting|CastToBP_NPC Actor)
    (:then
      (Default|TakeDamage _asbp_npc (Variables|Default|GetDamage))
      (Actor|DestroyActor)
      (return))
    (:CastFailed
      (Development|PrintString "NPC take damaged cast failed"))))

(fn HandleOtherOverlap
  (params (Actor :type Actor%20Object%20Reference))
  (if (or (== Actor "BP_PlayerProjectile_Child") (== Actor "/Game/FirstPerson/Blueprints/BP_Player.BP_Player"))
    _))