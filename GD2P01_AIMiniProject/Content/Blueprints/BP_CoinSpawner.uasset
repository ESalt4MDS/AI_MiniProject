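; BP_CoinSpawner is an actor that spawns BP_Coin at random points inside its Box component.
; BeginPlay starts SpawnCoin, which waits a random delay, spawns the coin and clears CanSpawn, a flag never read in this graph.
; When an actor tagged "Coin" ends overlap with the box, it prints a message, waits another random delay and calls SpawnCoin again, sustaining the respawn cycle.
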(event OnComponentEndOverlap(Box)
  (params (OverlappedComponent :type Primitive%20Component%20Object%20Reference) (OtherActor :type Actor%20Object%20Reference) (OtherComp :type Primitive%20Component%20Object%20Reference) (OtherBodyIndex :type Integer))
  (if (Actor|ActorHasTag OtherActor "Coin")
    (Development|PrintString "Coin gone")
    (Utilities|FlowControl|Delay (Math|Random|RandomFloatinRange 1.0 4.0))
    (CallFunction|SpawnCoin)))

(event Custom|SpawnCoin
  (bind _box (Variables|Default|GetBox))
  (Utilities|FlowControl|Delay (Math|Random|RandomFloatinRange 3.0 6.0))
  (Game|SpawnActorfromClass "/Game/Blueprints/BP_Coin.BP_Coin_C" (Math|Transform|MakeTransform (Math|Random|RandomPointinBoundingBox (Transformation|GetWorldLocation _box) (Variables|/Script/Engine.BoxComponent|GetBoxExtent _box)) "0, 0, 0" "1.000000,1.000000,1.000000") "AdjustIfPossibleButAlwaysSpawn" "MultiplyWithRoot" self 0)
  (Variables|Default|SetCanSpawn false))

(event EventBeginPlay
  (CallFunction|SpawnCoin))

(event Collision|EventActorBeginOverlap
  (params (OtherActor :type Actor%20Object%20Reference)))

(event EventTick
  (params (DeltaSeconds :type Float%20%28single-precision%29)))

(fn ConstructionScript)