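; AI controller for an NPC that runs BT_NPCTree and feeds its blackboard from perception.
; Sight sets the target actor, flags whether it is the player, and stores the player's last seen location; hearing sets a target location.
; Shoot spawns an enemy projectile ahead and restarts a cooldown that Tick counts down before setting CanShoot.
; A helper copies player health to the blackboard to drive behaviour changes.
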(event OnTargetPerceptionUpdated(AIPerception)
  (params (Actor :type Actor%20Object%20Reference) (Stimulus :type AI%20Stimulus%20Structure))
  (bind _returnvalue (Class|AIPerceptionSystem|GetSenseClassforStimulus Stimulus))
  (Utilities|FlowControl|Sequence
    (:then_0
      (if (== _returnvalue "/Script/AIModule.AISense_Sight")
        (CallFunction|HandleSight Actor Stimulus)))
    (:then_1
      (if (== _returnvalue "/Script/AIModule.AISense_Hearing")
        (CallFunction|HandleHearing Stimulus)))))

(event Custom|ShootDelay
  (params (Delta :type Float%20%28double-precision%29))
  (if (> (Variables|Default|GetShootDelayCount) 0.0)
    (bind _output_get (Variables|Default|SetShootDelayCount (- (Variables|Default|GetShootDelayCount) Delta)))
    (Development|PrintString (Utilities|String|ToString(Float) _output_get))
    (else
      (AI|Components|Blackboard|SetValueasBool (AI|GetBlackboard 0) (Utilities|Name|MakeLiteralName "CanShoot") true))))

(event EventBeginPlay
  (AI|RunBehaviorTree "/Game/NPC/BT_NPCTree.BT_NPCTree"))

(event EventTick
  (params (DeltaSeconds :type Float%20%28single-precision%29))
  (CallFunction|ShootDelay DeltaSeconds))

(fn ConstructionScript)

(fn HandleSight
  (params (Actor :type Actor%20Object%20Reference) (Stimulus :type AI%20Stimulus%20Structure))
  (bind (_age _expirationage _strength _stimuluslocation _receiverlocation _tag _bsuccessfullysensed) (Utilities|Struct|BreakAIStimulus Stimulus))
  (bind _returnvalue (AI|GetBlackboard 0))
  (bind _returnvalue_2 (AI|GetBlackboard 0))
  (if (== Actor (Game|GetPlayerCharacter 0))
    ;[0.15 0.15 0.15 0.5] IF NPC can see the player set the TargetActor for the NPC to stop and look at and IsPlayer is set to TRUE for the NPC to shoot at player
    (AI|Components|Blackboard|SetValueasObject _returnvalue_2 (Utilities|Name|MakeLiteralName "TargetActor") (Utilities|SelectObject Actor 0 _bsuccessfullysensed))
    (AI|Components|Blackboard|SetValueasBool _returnvalue_2 (Utilities|Name|MakeLiteralName "IsPlayer") true)
    ;[0.15 0.15 0.15 0.5] IF NPC can Not see player set the last seen location
    (if (not _bsuccessfullysensed)
      (AI|Components|Blackboard|SetValueasVector (AI|GetBlackboard 0) (Utilities|Name|MakeLiteralName "LastSeenLocation") _stimuluslocation))
    (else
      ;[0.15 0.15 0.15 0.5] IF NPC did Not see Player But Saw another Actor (Coin, Ammo) set that actor as the TargetActor for the NPC to move to and IsPlayer set to FALSE
      (AI|Components|Blackboard|SetValueasObject _returnvalue (Utilities|Name|MakeLiteralName "TargetActor") (Utilities|SelectObject Actor 0 _bsuccessfullysensed))
      (AI|Components|Blackboard|SetValueasBool _returnvalue (Utilities|Name|MakeLiteralName "IsPlayer") false))))

(fn Shoot
  (bind _worldtransform (Variables|Default|GetWorldTransform))
  ;[0.15 0.15 0.15 0.5] spawn and shoot where NPC is facing
  (Variables|Default|SetShootDelayCount (Variables|Default|GetMaxShootDelay))
  (Game|SpawnActorfromClass "/Game/Blueprints/BP_EnemyProjectile_Child.BP_EnemyProjectile_Child_C" (Math|Transform|MakeTransform (+ (.location _worldtransform) (* (Math|Vector|GetForwardVector (.rotation _worldtransform)) (LocalVariables|GetSpawnDistance))) (.rotation _worldtransform) "1.000000,1.000000,1.000000") "AlwaysSpawn" "MultiplyWithRoot" self 0))

(fn UpdatePlayerHealth
  (params (actor :type Actor%20Object%20Reference))
  ;[0.15 0.15 0.15 0.5] update player health to blackboard to be used for changing behaviour
  (bind _asbp_player (Utilities|Casting|CastToBP_Player actor))
  (AI|Components|Blackboard|SetValueasFloat (AI|GetBlackboard 0) (Utilities|Name|MakeLiteralName "PlayerHealth") (Variables|/Game/FirstPerson/Blueprints/BP_Player.BP_Player_C|GetHealth _asbp_player)))

(fn HandleHearing
  (params (Stimulus :type AI%20Stimulus%20Structure))
  (bind (_age _expirationage _strength _stimuluslocation _receiverlocation _tag _bsuccessfullysensed) (Utilities|Struct|BreakAIStimulus Stimulus))
  ;[0.15 0.15 0.15 0.5] when an actor is heard using AI Hearing set target location
  (if _bsuccessfullysensed
    (AI|Components|Blackboard|SetValueasVector (AI|GetBlackboard 0) (Utilities|Name|MakeLiteralName "TargetLocation") _stimuluslocation)))